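; BP_TimeSlowbility is a child ability Blueprint in SphereGame that, going by its name, grants the time-slow ability to the player's sphere.
; Its construction script sets the sphere material's Color to blue and applies it to the mesh.
; AddSomethingToPlayer calls the parent, sets the passed Sphere's CurrentAbility to an enum entry, and passes the material's color to SetSphereColor.
; The slowing effect itself is not implemented here.
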(event EventBeginPlay
  (|CallParentFunction))

(event Collision|EventActorBeginOverlap
  (params (OtherActor :type Actor%20Object%20Reference))
  (|CallParentFunction OtherActor) ; This node is disabled and will not be called.\nDrag off pins to build functionality.
)

(event EventTick
  (params (DeltaSeconds :type Float%20%28single-precision%29))
  (|CallParentFunction DeltaSeconds) ; This node is disabled and will not be called.\nDrag off pins to build functionality.
)

(fn ConstructionScript
  (bind _spherematerial (Variables|Default|GetSphereMaterial))
  (|CallParentFunction)
  (Rendering|Material|SetVectorParameterValue _spherematerial "Color" "(R=0.000000,G=0.101227,B=1.000000,A=1.000000)" :!class /Script/Engine.MaterialInstanceDynamic)
  (Rendering|Material|SetMaterial (Variables|Default|GetSphere) 0 _spherematerial))

(fn AddSomethingtoPlayer
  (params (Sphere :type BP%20Sphere%20Player%20Object%20Reference))
  (|CallParentFunction Sphere)
  (Variables|/Game/SphereGame/BP_SpherePlayer.BP_SpherePlayer_C|SetCurrentAbility Sphere "NewEnumerator0")
  (bind _returnvalue (Rendering|Material|GetVectorParameterValue (Variables|Default|GetSphereMaterial) "Color" :!class /Script/Engine.MaterialInstanceDynamic))
  (Default|SetSphereColor Sphere _returnvalue))