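; BP_AbilitySphere is a pickup sphere for BP_SpherePlayer, apparently a template for granting an ability, but its pickup logic is unfinished.
; Tick counts up a timer and, past SpawnTime, keeps the sphere visible and collidable.
; The overlap event only casts to the player; the empty AddSomethingToPlayer hook and the hide-and-reset respawn steps are disconnected.
; The construction script creates a dynamic material instance from MI_SphereMaterial.
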(event OnComponentBeginOverlap(SphereCollision)
  (params (OverlappedComponent :type Primitive%20Component%20Object%20Reference) (OtherActor :type Actor%20Object%20Reference) (OtherComp :type Primitive%20Component%20Object%20Reference) (OtherBodyIndex :type Integer) (bFromSweep :type Boolean) (SweepResult :type Hit%20Result%20Structure%20%28by%20ref%29))
  (bind _asbp_sphere_player (Utilities|Casting|CastToBP_SpherePlayer OtherActor)))

(event EventBeginPlay)

(event Collision|EventActorBeginOverlap
  (params (OtherActor :type Actor%20Object%20Reference)))

(event EventTick
  (params (DeltaSeconds :type Float%20%28single-precision%29))
  (bind _output_get (Variables|Default|SetTimer (+ (Variables|Default|GetTimer) DeltaSeconds)))
  (if (>= _output_get (Variables|Default|GetSpawnTime))
    (Rendering|SetActorHiddenInGame false)
    (Collision|SetActorEnableCollision true)))

(fn ConstructionScript
  (bind _returnvalue (Rendering|Material|CreateDynamicMaterialInstance "/Game/SphereGame/Material/MI_SphereMaterial.MI_SphereMaterial" "None" "None" :!class /Script/Engine.KismetMaterialLibrary))
  (Variables|Default|SetSphereMaterial _returnvalue))

(fn AddSomethingtoPlayer
  (params (Sphere :type BP%20Sphere%20Player%20Object%20Reference)))