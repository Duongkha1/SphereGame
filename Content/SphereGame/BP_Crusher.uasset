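; BP_Crusher is a moving hazard that sends BP_SpherePlayer back to its starting position when it overlaps the Cube.
; Tick accumulates a timer and applies a sine math expression, scaled by delta time and Height, as a local Z offset to move it up and down.
; The construction script gives the Cube a red dynamic instance of BasicShapeMaterial.
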(event OnComponentBeginOverlap(Cube)
  (params (OverlappedComponent :type Primitive%20Component%20Object%20Reference) (OtherActor :type Actor%20Object%20Reference) (OtherComp :type Primitive%20Component%20Object%20Reference) (OtherBodyIndex :type Integer) (bFromSweep :type Boolean) (SweepResult :type Hit%20Result%20Structure%20%28by%20ref%29))
  (bind _asbp_sphere_player (Utilities|Casting|CastToBP_SpherePlayer OtherActor))
  (Default|TeleporttoStartingPosition _asbp_sphere_player))

(event EventBeginPlay)

(event Collision|EventActorBeginOverlap
  (params (OtherActor :type Actor%20Object%20Reference)))

(event EventTick
  (params (DeltaSeconds :type Float%20%28single-precision%29))
  (Variables|Default|SetTimer (+ DeltaSeconds (Variables|Default|GetTimer)))
  (Transformation|AddActorLocalOffset (Math|Vector|MakeVector 0.0 0.0 (* (|((Sin(({715BC270-4C9D-B444-7453-009F0BAE770E}*{5B0BB813-42DF-B947-8B86-51856DCB6748})))*{C4710A8D-47C7-0FC9-FA05-C6947AB6D2B7})) DeltaSeconds (Variables|Default|GetHeight))) false false))

(fn ConstructionScript
  (bind _returnvalue (Rendering|Material|CreateDynamicMaterialInstance "/Engine/BasicShapes/BasicShapeMaterial.BasicShapeMaterial" "None" "None" :!class /Script/Engine.KismetMaterialLibrary))
  (bind _output_get (Variables|Default|SetSphereMaterial _returnvalue))
  (Rendering|Material|SetVectorParameterValue _output_get "Color" "(R=1.000000,G=0.019020,B=0.000000,A=1.000000)" :!class /Script/Engine.MaterialInstanceDynamic)
  (Rendering|Material|SetMaterial (Variables|Default|GetCube) 0 _output_get))