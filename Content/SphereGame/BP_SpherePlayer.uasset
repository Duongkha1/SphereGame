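; Player-controlled sphere for SphereGame that moves along its forward vector and turns in 90-degree steps through Enhanced Input.
; The ability input consumes CurrentAbility; Levitation, the only one handled, instantly offsets the actor upward, then SetAbilityProperties clears the slot and starts a timer.
; Tick drops the IsAbilityActive flag after five seconds.
; SetSphereColor writes to a dynamic material created at BeginPlay, which this graph never assigns to the mesh.
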(event Input|EnhancedActionEvents|EnhancedInputActionIA_SphereMove
  (params (ActionValue :type Float%20%28double-precision%29) (ElapsedSeconds :type Float%20%28double-precision%29) (TriggeredSeconds :type Float%20%28double-precision%29) (InputAction :type Input%20Action%20Object%20Reference :default "/Game/SphereGame/Input/IA_SphereMove.IA_SphereMove"))
  (Pawn|Input|AddMovementInput (Transformation|GetActorForwardVector) (* ActionValue (Variables|Default|GetSpeed)) false))

(event Input|EnhancedActionEvents|EnhancedInputActionIA_SphereRotate
  (params (ActionValue :type Float%20%28double-precision%29) (ElapsedSeconds :type Float%20%28double-precision%29) (TriggeredSeconds :type Float%20%28double-precision%29) (InputAction :type Input%20Action%20Object%20Reference :default "/Game/SphereGame/Input/IA_SphereRotate.IA_SphereRotate"))
  (:Started
    (Transformation|AddActorLocalRotation (Math|Rotator|MakeRotator 0.0 0.0 (* (Math|Float|Sign(Float) ActionValue) 9e+01)) false false)))

(event Input|EnhancedActionEvents|EnhancedInputActionIA_SphereActivateAbility
  (params (ActionValue :type Boolean) (ElapsedSeconds :type Float%20%28double-precision%29) (TriggeredSeconds :type Float%20%28double-precision%29) (InputAction :type Input%20Action%20Object%20Reference :default "/Game/SphereGame/Input/IA_SphereActivateAbility.IA_SphereActivateAbility"))
  (:Started
    (switch Utilities|FlowControl|Switch|SwitchonE_Abilities (Variables|Default|GetCurrentAbility)
      (:NewEnumerator1
        (Transformation|AddActorLocalOffset "0.000000,0.000000,300.000000" false false)
        (CallFunction|SetAbilityProperties)))))

(event EventBeginPlay
  (Input|AddMappingContext (PlayerController|LocalPlayerSubsystems|GetEnhancedInputLocalPlayerSubsystem (Game|GetPlayerController 0)) "/Game/SphereGame/Input/IMC_SphereCharacter.IMC_SphereCharacter" 0 "(bIgnoreAllPressedKeysUntilRelease=True,bForceImmediately=False,bNotifyUserSettings=False)")
  (bind _returnvalue (Rendering|Material|CreateDynamicMaterialInstance (Rendering|Material|GetMaterial (Variables|Default|GetSphere) 0) "None" "None" :!class /Script/Engine.KismetMaterialLibrary))
  (Variables|Default|SetDynamicMaterial _returnvalue))

(event Collision|EventActorBeginOverlap
  (params (OtherActor :type Actor%20Object%20Reference)))

(event EventTick
  (params (DeltaSeconds :type Float%20%28single-precision%29))
  (bind _output_get (Variables|Default|SetAbilityTimer (+ DeltaSeconds (Variables|Default|GetAbilityTimer))))
  (if (>= _output_get 5.0)
    (Variables|Default|SetIsAbilityActive false)))

(fn ConstructionScript)

(fn SetAbilityProperties
  (Variables|Default|SetCurrentAbility "NewEnumerator0")
  (Variables|Default|SetAbilityTimer 0.0)
  (Variables|Default|SetIsAbilityActive true))

(fn SetSphereColor
  (params (Color :type Linear%20Color%20Structure))
  (Rendering|Material|SetVectorParameterValue (Variables|Default|GetDynamicMaterial) "Color" Color :!class /Script/Engine.MaterialInstanceDynamic))